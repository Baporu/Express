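; Short-lived smoke puff actor that drifts upward and then removes itself.
; On BeginPlay it randomizes its scale and its rotation on all three axes, then destroys itself after a brief delay.
; Tick raises it by a fixed step along world Z every frame without using delta time, so the rise speed depends on frame rate.
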(event EventBeginPlay
  (bind _returnvalue (Math|Random|RandomFloatinRange 0.0 3.6e+02))
  (Transformation|SetActorScale3D (+ (Variables|Default|GetNew%20Scale%203D) (Math|Random|RandomFloatinRange 0.2 0.5)))
  (Transformation|SetActorRotation (Math|Rotator|MakeRotator _returnvalue _returnvalue _returnvalue))
  (Utilities|FlowControl|Delay 1.2)
  (Actor|DestroyActor))

(event Collision|EventActorBeginOverlap
  (params (OtherActor :type Actor%20Object%20Reference)))

(event EventTick
  (params (DeltaSeconds :type Float%20%28single-precision%29))
  (Transformation|SetActorLocation (+ (Transformation|GetActorLocation) "0.000000,0.000000,1.000000") false false))

(fn ConstructionScript)